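; BP_BaseAI_Chase is a base AI enemy that chases the top-down player character and knocks it back on contact.
; Pawn sensing starts an AI MoveTo targeting any BP_TopDownCharacter it sees.
; A box collision overlap launches the player along the direction away from the enemy's capsule, scaled by LaunchVelocity, and plays a pop sound at the world origin.
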(event OnComponentBeginOverlap(BoxCollision)
  (params (OverlappedComponent :type Primitive%20Component%20Object%20Reference) (OtherActor :type Actor%20Object%20Reference) (OtherComp :type Primitive%20Component%20Object%20Reference) (OtherBodyIndex :type Integer) (bFromSweep :type Boolean) (SweepResult :type Hit%20Result%20Structure%20%28by%20ref%29))
  ;[1 1 1] When player his hit by enemy the player is pushed back from Launch Velocity
  (bind _asbp_top_down_character (Utilities|Casting|CastToBP_TopDownCharacter OtherActor))
  (Character|LaunchCharacter _asbp_top_down_character (* (Math|Vector|GetUnitDirection(Vector) (Transformation|GetWorldLocation (Variables|Default|GetCapsuleComponent)) (Transformation|GetActorLocation _asbp_top_down_character)) (Variables|Default|GetLaunchVelocity)) false false)
  (Audio|PlaySoundatLocation "/Game/Audio/Interface_And_Item_Sounds/WAV/Abstract_Pop_04.Abstract_Pop_04" "0, 0, 0" "0, 0, 0" 1.0 1.0 0.0 0 0 0 0))

(event OnSeePawn(PawnSensing)
  (params (Pawn :type Pawn%20Object%20Reference))
  (bind _asbp_top_down_character (Utilities|Casting|CastToBP_TopDownCharacter Pawn))
  (AI|AIMoveTo self (Transformation|GetActorLocation) _asbp_top_down_character 5.0 false))

(event EventBeginPlay)

(event Collision|EventActorBeginOverlap
  (params (OtherActor :type Actor%20Object%20Reference)))

(event EventTick
  (params (DeltaSeconds :type Float%20%28single-precision%29)))

(fn ConstructionScript
  (|CallParentFunction))