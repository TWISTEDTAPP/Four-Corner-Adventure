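; Base AI Blueprint with a KnockBack event that pushes its mesh along the player character's control-rotation forward vector.
; KnockBack switches the mesh to the Ragdoll profile but sets physics simulation off, then applies a velocity-change impulse and disables the box's collision.
; RotateToFaceCursor and the construction script are empty, with cursor-trace and look-at nodes left unconnected.
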(event Custom|KnockBack
  (bind _mesh (Variables|Character|GetMesh))
  (Collision|SetCollisionProfileName _mesh "Ragdoll" true :!class /Script/Engine.PrimitiveComponent)
  (Physics|SetSimulatePhysics _mesh false)
  (bind _asbp_top_down_character (Utilities|Casting|CastToBP_TopDownCharacter (Game|GetPlayerCharacter 0)))
  (Physics|AddImpulse (Variables|Character|GetMesh) (* (Math|Vector|GetForwardVector (Pawn|GetControlRotation _asbp_top_down_character :!class /Script/Engine.Pawn)) 3e+03) "None" true)
  (Collision|SetCollisionEnabled (Variables|Default|GetBoxCollision) "NoCollision"))

(fn ConstructionScript)

(fn RotatetoFaceCursor)